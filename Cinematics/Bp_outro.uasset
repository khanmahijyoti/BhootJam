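; Outro trigger actor that ends the game with a cinematic and a return to the menu.
; When the HorrorEngineCharacter overlaps it, it plays the FinalOutro level sequence and disables player move and look input.
; After a fixed delay it opens the menu level.
; A disconnected branch that would restore input and destroy the actor never runs.
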(event `self.ReceiveActorBeginOverlap`
  (params (OtherActor :type "Actor Object Reference"))
  (bind _returnvalue (`GameplayStatics.GetPlayerController` 0))
  (bind _ashorror_engine_character (cast `/Game/HorrorEngine/Blueprints/Core/HorrorEngineCharacter` OtherActor))
  (bind (_outactor _returnvalue_2) (`LevelSequencePlayer.CreateLevelSequencePlayer` "/Game/Cinematics/FinalOutro.FinalOutro"))
  (`MovieSceneSequencePlayer.Play` _returnvalue_2)
  (`Controller.SetIgnoreMoveInput` _returnvalue true)
  (`Controller.SetIgnoreLookInput` _returnvalue true)
  (`KismetSystemLibrary.Delay` 5.0)
  (`GameplayStatics.OpenLevelBySoftObjectPtr` "/Game/HorrorEngine/Maps/MenuLevel.MenuLevel"))

(fn `UserConstructionScript`)
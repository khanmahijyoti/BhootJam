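; BP_BasketballGround is a one-shot trigger actor that plays a basketball cinematic when something overlaps it.
; A DoOnce gates the first overlap, which must be a HorrorEngineCharacter for the MysequenceBasketball level sequence to play.
; Player move and look input are ignored for a fixed delay, then restored, and the actor destroys itself after a further wait.
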(event `self.ReceiveActorBeginOverlap`
  (params (OtherActor :type "Actor Object Reference"))
  (bind _returnvalue (`GameplayStatics.GetPlayerController` 0))
  (bind _returnvalue_2 (`GameplayStatics.GetPlayerController` 0))
  (`/Engine/EditorBlueprintResources/StandardMacros.DoOnce` false
    (:`Completed`
      (bind _ashorror_engine_character (cast `/Game/HorrorEngine/Blueprints/Core/HorrorEngineCharacter` OtherActor))
      (bind (_outactor _returnvalue_3) (`LevelSequencePlayer.CreateLevelSequencePlayer` (`self.MysequenceBasketball`)))
      (`MovieSceneSequencePlayer.Play` _returnvalue_3)
      (`Controller.SetIgnoreMoveInput` _returnvalue true)
      (`Controller.SetIgnoreLookInput` _returnvalue true)
      (`KismetSystemLibrary.Delay` 5.0)
      (`Controller.SetIgnoreMoveInput` _returnvalue_2 false)
      (`Controller.SetIgnoreLookInput` _returnvalue_2 false)
      (`KismetSystemLibrary.Delay` 5.0)
      (`self.K2_DestroyActor`))))

(fn `UserConstructionScript`)